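; BP_Inventory is an inventory Blueprint that sorts its Items array in ascending order of each item's Value using a hand-written merge sort.
; SortItemsByValue starts the recursion over the whole array, and SortItemArrayPartByValue halves each range until it holds one element or none.
; MergeTwoArrayPartsSortedByValue copies both halves into local arrays, then writes the smaller front item back into Items, taking the right one on ties.
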(fn MergeTwoArrayPartsSortedbyValue
  (params (LeftBorder :type Integer) (MidBorder :type Integer) (RightBorder :type Integer))
  (LocalVariables|SetLocal_LeftBorder LeftBorder)
  (LocalVariables|SetLocal_MidBorder MidBorder)
  (LocalVariables|SetLocal_RightBorder RightBorder)
  ;[1 1 1] Isolating left part
  (for _index (range (LocalVariables|GetLocal_LeftBorder) (LocalVariables|GetLocal_MidBorder))
    (Utilities|Array|Add (LocalVariables|GetLocal_LeftPart) (Utilities|Array|Get(acopy) (Variables|Default|GetItems) _index)))
  ;[1 1 1] Isolating right part
  (for _index_2 (range (+ (LocalVariables|GetLocal_MidBorder) 1) (LocalVariables|GetLocal_RightBorder))
    (Utilities|Array|Add (LocalVariables|GetLocal_RightPart) (Utilities|Array|Get(acopy) (Variables|Default|GetItems) _index_2)))
  (LocalVariables|SetLocal_CurrentLeftItemIndex 0)
  (LocalVariables|SetLocal_CurrentRightItemIndex 0)
  (LocalVariables|SetLocal_CurrentMainIndex (LocalVariables|GetLocal_LeftBorder))
  (while (and (< (LocalVariables|GetLocal_CurrentLeftItemIndex) (Utilities|Array|Length (LocalVariables|GetLocal_LeftPart))) (< (LocalVariables|GetLocal_CurrentRightItemIndex) (Utilities|Array|Length (LocalVariables|GetLocal_RightPart))))
    (if (< (.Value (Utilities|Struct|BreakInventoryItem (Utilities|Array|Get(acopy) (LocalVariables|GetLocal_LeftPart) (LocalVariables|GetLocal_CurrentLeftItemIndex)))) (.Value (Utilities|Struct|BreakInventoryItem (Utilities|Array|Get(acopy) (LocalVariables|GetLocal_RightPart) (LocalVariables|GetLocal_CurrentRightItemIndex)))))
      (Utilities|Array|SetArrayElem (Variables|Default|GetItems) (LocalVariables|GetLocal_CurrentMainIndex) (Utilities|Array|Get(acopy) (LocalVariables|GetLocal_LeftPart) (LocalVariables|GetLocal_CurrentLeftItemIndex)))
      (Math|Integer|IncrementInt (LocalVariables|GetLocal_CurrentLeftItemIndex)
        (:%20%20
          (Math|Integer|IncrementInt (LocalVariables|GetLocal_CurrentMainIndex))))
      (else
        (Utilities|Array|SetArrayElem (Variables|Default|GetItems) (LocalVariables|GetLocal_CurrentMainIndex) (Utilities|Array|Get(acopy) (LocalVariables|GetLocal_RightPart) (LocalVariables|GetLocal_CurrentRightItemIndex)))
        (Math|Integer|IncrementInt (LocalVariables|GetLocal_CurrentRightItemIndex)
          (:%20%20
            (Math|Integer|IncrementInt (LocalVariables|GetLocal_CurrentMainIndex)))))))
  ;[1 1 1] Copying the remaining left part elements
  (while (< (LocalVariables|GetLocal_CurrentLeftItemIndex) (Utilities|Array|Length (LocalVariables|GetLocal_LeftPart)))
    (Utilities|Array|SetArrayElem (Variables|Default|GetItems) (LocalVariables|GetLocal_CurrentMainIndex) (Utilities|Array|Get(acopy) (LocalVariables|GetLocal_LeftPart) (LocalVariables|GetLocal_CurrentLeftItemIndex)))
    (Math|Integer|IncrementInt (LocalVariables|GetLocal_CurrentLeftItemIndex)
      (:%20%20
        (Math|Integer|IncrementInt (LocalVariables|GetLocal_CurrentMainIndex)))))
  ;[1 1 1] Copying the remaining right part elements
  (while (< (LocalVariables|GetLocal_CurrentRightItemIndex) (Utilities|Array|Length (LocalVariables|GetLocal_RightPart)))
    (Utilities|Array|SetArrayElem (Variables|Default|GetItems) (LocalVariables|GetLocal_CurrentMainIndex) (Utilities|Array|Get(acopy) (LocalVariables|GetLocal_RightPart) (LocalVariables|GetLocal_CurrentRightItemIndex)))
    (Math|Integer|IncrementInt (LocalVariables|GetLocal_CurrentRightItemIndex)
      (:%20%20
        (Math|Integer|IncrementInt (LocalVariables|GetLocal_CurrentMainIndex))))))

(fn SortItemArrayPartbyValue
  (params (LeftBorder :type Integer) (RightBorder :type Integer))
  (LocalVariables|SetLocal_LeftBorder LeftBorder)
  (LocalVariables|SetLocal_RightBorder RightBorder)
  (if (<= (LocalVariables|GetLocal_RightBorder) (LocalVariables|GetLocal_LeftBorder))
    (return)
    (else
      (LocalVariables|SetLocal_MidBorder (/ (+ (LocalVariables|GetLocal_RightBorder) (LocalVariables|GetLocal_LeftBorder)) 2))
      (CallFunction|SortItemArrayPartbyValue (LocalVariables|GetLocal_LeftBorder) (LocalVariables|GetLocal_MidBorder))
      (CallFunction|SortItemArrayPartbyValue (+ (LocalVariables|GetLocal_MidBorder) 1) (LocalVariables|GetLocal_RightBorder))
      (CallFunction|MergeTwoArrayPartsSortedbyValue (LocalVariables|GetLocal_LeftBorder) (LocalVariables|GetLocal_MidBorder) (LocalVariables|GetLocal_RightBorder)))))

(fn SortItemsbyValue
  (CallFunction|SortItemArrayPartbyValue 0 (- (Utilities|Array|Length (Variables|Default|GetItems)) 1)))